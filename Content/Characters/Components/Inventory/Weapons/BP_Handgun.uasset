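; Handgun weapon Blueprint that fires one projectile each time firing starts, as long as the magazine is not empty.
; Each shot decrements the magazine, plays the shot sound and spawns a HandgunProjectile with weapon damage and the owner pawn's velocity.
; A shared transform helper combines the HandgunSocket position, offset forward and up, with the view rotation.
; Tick projects a point derived from that transform to the screen to position the crosshair created at BeginPlay.
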(event `self.ReceiveBeginPlay`
  (`parent.ReceiveBeginPlay`)
  ;[1 1 1] create crosshair
  (bind _returnvalue (`|CreateWidget` "/Game/Characters/Components/Inventory/Weapons/crosshair.crosshair_C"))
  (set `self.crosshairRef` _returnvalue)
  (bind _aspawn (cast `Pawn` (`self.GetOwner`)))
  (set `self.OwnerPawn` _aspawn))

(event `self.ReceiveTick`
  (params (DeltaSeconds :type "Float (single-precision)"))
  ;[1 1 1] set crosshair position
  (bind _transform (`self.getProjectileTransform`))
  (`UserWidget.SetPositionInViewport` (`self.crosshairRef`) (`GameplayStatics.ProjectWorldToScreen` (`GameplayStatics.GetPlayerController` 0) (+ (.location _transform) (* (.rotation _transform) 500.0))) true))

(fn `Fire`
  (bind _ownerpawn (`self.OwnerPawn`))
  (`parent.Fire`)
  (if (not (`self.IsEmptyMag`))
    (`self.DecrementMagazine`)
    (`GameplayStatics.PlaySound2D` (`/Game/Characters/Components/Inventory/Weapons/WeaponDataAsset.ShotSound` (`self.WeaponData`)) 1.0 1.0 0.0 null null false)
    ;[1 1 1] create projectile
    (bind _transform (`self.getProjectileTransform`))
    (`|SpawnActorFromClass` "/Game/Fab/Particles/handgunProjectile.handgunProjectile_C" _transform "Undefined" "MultiplyWithRoot" null (`/Game/Characters/Components/Inventory/Weapons/WeaponDataAsset.Damage` (`self.WeaponData`)) (`MovementComponent.Velocity` (`Pawn.GetMovementComponent` _ownerpawn)) _ownerpawn)))

(fn `getProjectileTransform`
  (returns (transform :type "Transform Structure"))
  (bind (_outlocation _outrotation) (`Actor.GetActorEyesViewPoint` (`Controller.K2_GetPawn` (`GameplayStatics.GetPlayerController` 0))))
  (return (`KismetMathLibrary.MakeTransform` (+ (+ (`self.GetSocketLocation` (`Character.Mesh` (`GameplayStatics.GetPlayerCharacter` 0)) "HandgunSocket") (* (`KismetMathLibrary.Normal` (`KismetMathLibrary.Conv_RotatorToVector` _outrotation)) (20.0 20.0 20.0))) (0.0 0.0 10.0)) _outrotation)))

(fn `StartFiring`
  (`parent.StartFiring`)
  (`self.Fire`))