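; BP_WeaponPickUp is a world pickup that gives a weapon to the player robot when interacted with.
; The construction script sets its static mesh from the weapon data in its WeaponSlot.
; Hint events show or hide its widget, and Interact adds the slot to the PlayerRobotCharacter's InventoryComponent, then destroys the pickup.
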(event `/Game/Characters/Components/Interaction/InteractableInterface.HideHint`
  (`SceneComponent.SetVisibility` (`self.Widget`) false false))

(event `/Game/Characters/Components/Interaction/InteractableInterface.ShowHint`
  (`SceneComponent.SetVisibility` (`self.Widget`) true false))

(event `/Game/Characters/Components/Interaction/InteractableInterface.Interact`
  (params (WithActor :type "Actor Object Reference"))
  (bind _asplayer_robot_character (cast `/Game/Characters/PlayerRobotCharacter` WithActor))
  (`/Game/Characters/Components/Inventory/InventoryComponent.AddWeaponToInventory` (`/Game/Characters/PlayerRobotCharacter.InventoryComponent` _asplayer_robot_character) (`self.WeaponSlot`))
  (`self.K2_DestroyActor`))

(fn `UserConstructionScript`
  (`parent.UserConstructionScript`)
  (`StaticMeshComponent.SetStaticMesh` (`self.StaticMesh`) (`/Game/Characters/Components/Inventory/Weapons/WeaponDataAsset.Mesh` (`.WeaponData_2_80FE8EB04A3BA93657F65E81FEC6ED8F` (break `/Game/Characters/Components/Inventory/Weapons/WeaponSlotStruct` (`self.WeaponSlot`))))))