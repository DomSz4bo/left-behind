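; Base weapon Blueprint that sets its static mesh from WeaponData and manages reserve and magazine ammo.
; Reload moves as much reserve ammo as fits in the magazine and returns whether any was added.
; DecrementMagazine and Reload broadcast ammo changes through event dispatchers, and IsEmptyMag reports an empty magazine.
; StartFiring and StopFiring only print debug text, and Fire is an empty stub.
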(event `self.ReceiveBeginPlay`
  (`self.SetStaticMesh` (`/Game/Characters/Components/Inventory/Weapons/WeaponDataAsset.Mesh` (`self.WeaponData`))))

(fn `DecrementMagazine`
  (bind _result (`/Engine/EditorBlueprintResources/StandardMacros.DecrementInt` (`self.InMagazineAmmo`))
    (:`  `
      (`self.OnMagAmountChange` _result))))

(fn `Fire`)

(fn `IsEmptyMag`
  (returns (EmptyMag :type Boolean))
  (return (== (`self.InMagazineAmmo`) 0)))

(fn `Reload`
  (returns (ReloadSuccess :type Boolean))
  (locals (AddToMagazineAmount :type Integer))
  (`KismetSystemLibrary.PrintString` "Reload")
  (if (not (== (`self.Ammo`) 0))
    (bind _output_get (set `local.AddToMagazineAmount` (`KismetMathLibrary.Clamp` (- (`/Game/Characters/Components/Inventory/Weapons/WeaponDataAsset.MagazineCapacity` (`self.WeaponData`)) (`self.InMagazineAmmo`)) 0 (`self.Ammo`))))
    (if (== _output_get 0)
      _
      (else
        (bind _output_get_2 (set `self.Ammo` (- (`self.Ammo`) (`local.AddToMagazineAmount`))))
        (`self.OnAmmoAmountChange` _output_get_2)
        (bind _output_get_3 (set `self.InMagazineAmmo` (+ (`local.AddToMagazineAmount`) (`self.InMagazineAmmo`))))
        (`self.OnMagAmountChange` _output_get_3)
        (return true))))
  (return false))

(fn `StartFiring`
  (`KismetSystemLibrary.PrintString` "Start Firing"))

(fn `StopFiring`
  (`KismetSystemLibrary.PrintString` "Stop Firing"))