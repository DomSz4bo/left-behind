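; ConsumableItem_BP is a world pickup for a consumable item that the player robot can collect into its inventory.
; The construction script sets the static mesh and its scale from ConsumableData.
; On Interact, it passes ConsumableData to the PlayerRobotCharacter's InventoryComponent and destroys itself only if the add succeeds.
; ShowHint and HideHint toggle the visibility of its interaction widget.
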(event `/Game/Characters/Components/Interaction/InteractableInterface.Interact`
  (params (WithActor :type "Actor Object Reference"))
  (bind _asplayer_robot_character_2 (cast `/Game/Characters/PlayerRobotCharacter` WithActor))
  (bind _addedsuccessfully (`/Game/Characters/Components/Inventory/InventoryComponent.AddConsumableToInventory` (`/Game/Characters/PlayerRobotCharacter.InventoryComponent` _asplayer_robot_character_2) (`self.ConsumableData`)))
  (if _addedsuccessfully
    (`self.K2_DestroyActor`)))

(event `/Game/Characters/Components/Interaction/InteractableInterface.ShowHint`
  (`self.ShowInteractionWidget`))

(event `/Game/Characters/Components/Interaction/InteractableInterface.HideHint`
  (`self.HideInteractionWodget`))

(fn `HideInteractionWodget`
  (`SceneComponent.SetVisibility` (`self.Widget`) false false))

(fn `ShowInteractionWidget`
  (`SceneComponent.SetVisibility` (`self.Widget`) true false))

(fn `UserConstructionScript`
  (`StaticMeshComponent.SetStaticMesh` (`self.StaticMesh`) (`/Game/Characters/Components/Inventory/Consumables/ConsumableItemDataAsset.Mesh` (`self.ConsumableData`)))
  (`SceneComponent.SetRelativeScale3D` (`self.StaticMesh`) (`/Game/Characters/Components/Inventory/Consumables/ConsumableItemDataAsset.MeshScale` (`self.ConsumableData`))))