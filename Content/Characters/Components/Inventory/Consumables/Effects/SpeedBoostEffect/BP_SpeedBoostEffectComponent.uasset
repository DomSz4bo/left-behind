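; Actor component that applies a temporary speed boost consumable effect to the player robot character.
; On BeginPlay it casts its owner to PlayerRobotCharacter, scales the max running speed by a multiplier and starts a duration timer.
; When the timer ends it resets the running speed, destroys itself and prints an end-of-effect message.
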(event `self.ReceiveBeginPlay`
  (bind _asplayer_robot_character_2 (cast `/Game/Characters/PlayerRobotCharacter` (`self.GetOwner`)))
  (bind _output_get (set `self.OwnerCharacter` _asplayer_robot_character_2))
  (`/Game/Characters/PlayerRobotCharacter.SetMaxRunningSpeed` _output_get (* (`/Game/Characters/PlayerRobotCharacter.MaxRunningSpeed` _output_get) (`self.MaxRunSpeedMultiplier`)))
  (`self.SetTimer`))

(event `TimerEnd`
  (`/Game/Characters/PlayerRobotCharacter.ResetMaxRunningSpeed` (`self.OwnerCharacter`))
  (`self.K2_DestroyComponent`)
  (`KismetSystemLibrary.PrintString` "EndOfEffect"))

(fn `SetTimer`
  (`KismetSystemLibrary.K2_SetTimerDelegate` (`|CreateDelegate` :!event `TimerEnd`) (`self.DurationSeconds`)))