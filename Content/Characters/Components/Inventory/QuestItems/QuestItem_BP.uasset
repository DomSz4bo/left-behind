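; Quest item pickup actor that takes its mesh and scale from QuestItemData in the construction script.
; ShowHint and HideHint events toggle the visibility of its interaction widget.
; The Interact event is empty, and the logic that adds the item to the inventory and destroys the actor on success is not connected to any event.
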(event `/Game/Characters/Components/Interaction/InteractableInterface.Interact`
  (params (WithActor :type "Actor Object Reference")))

(event `/Game/Characters/Components/Interaction/InteractableInterface.ShowHint`
  (`self.ShowInteractionWidget`))

(event `/Game/Characters/Components/Interaction/InteractableInterface.HideHint`
  (`self.HideInteractionWidget`))

(fn `HideInteractionWidget`
  (`SceneComponent.SetVisibility` (`self.Widget`) false false))

(fn `ShowInteractionWidget`
  (`SceneComponent.SetVisibility` (`self.Widget`) true false))

(fn `UserConstructionScript`
  (`parent.UserConstructionScript`)
  (`StaticMeshComponent.SetStaticMesh` (`self.StaticMesh`) (`/Game/Characters/Components/Inventory/QuestItems/QuestItemDataAsset.Mesh` (`self.QuestItemData`)))
  (`SceneComponent.SetRelativeScale3D` (`self.StaticMesh`) (`/Game/Characters/Components/Inventory/QuestItems/QuestItemDataAsset.MeshScale` (`self.QuestItemData`))))