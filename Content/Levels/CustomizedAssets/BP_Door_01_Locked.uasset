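; Locked sliding door that the player robot unlocks with a quest key item from its inventory.
; Interacting consumes single-use keys, swaps access panel materials, fires OnDoorUnlocked and opens the door; failure shows a message and error sound.
; Once unlocked, box overlaps play or reverse the slide timeline that lerps both panels.
; A widget shows the locked hint, and the construction script applies the door material.
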(event `self.Box.OnComponentBeginOverlap`
  (params (OverlappedComponent :type "PrimitiveComponent Object Reference") (OtherActor :type "Actor Object Reference") (OtherComp :type "PrimitiveComponent Object Reference") (OtherBodyIndex :type Integer) (bFromSweep :type Boolean) (SweepResult :type "HitResult Structure (by ref)"))
  (if (`self.Unlocked`)
    (`self.OpenDoors`)))

(event `self.Box.OnComponentEndOverlap`
  (params (OverlappedComponent :type "PrimitiveComponent Object Reference") (OtherActor :type "Actor Object Reference") (OtherComp :type "PrimitiveComponent Object Reference") (OtherBodyIndex :type Integer))
  (`self.CloseDoors`))

(event `/Game/Characters/Components/Interaction/InteractableInterface.HideHint`
  (`self.HideHintWidget `))

(event `/Game/Characters/Components/Interaction/InteractableInterface.ShowHint`
  (if (not (`self.Unlocked`))
    (`self.ShowUnlockHint`)))

(event `/Game/Characters/Components/Interaction/InteractableInterface.Interact`
  (params (WithActor :type "Actor Object Reference"))
  (if (not (`self.Unlocked`))
    (bind _asplayer_robot_character (cast `/Game/Characters/PlayerRobotCharacter` WithActor))
    (bind _unlocksuccess (`self.UnlockWithKey` (`/Game/Characters/PlayerRobotCharacter.InventoryComponent` _asplayer_robot_character)))
    (if _unlocksuccess
      (`self.OpenDoors`)
      (`self.HideHintWidget `)
      (else
        (`self.ShowUnlockFail`)
        (`GameplayStatics.PlaySound2D` "/Game/SoundEffects/8-bit-error.8-bit-error" 1.0 1.0 0.0 null null false)))))

(event `self.ReceiveBeginPlay`
  (bind _aswbp_interaction_hint (cast `/Game/Characters/Components/Interaction/WBP_InteractionHint` (`WidgetComponent.GetWidget` (`self.Widget`))))
  (set `self.HintWidget` _aswbp_interaction_hint))

(fn `CloseDoors`
  (`TimelineComponent.Reverse` (`self.Door_Slide`)))

(fn `HideHintWidget `
  (`SceneComponent.SetVisibility` (`self.Widget`) false false))

(fn `OpenDoors`
  (`TimelineComponent.Play` (`self.Door_Slide`)))

(fn `ShowUnlockFail`
  (`SceneComponent.SetVisibility` (`self.Widget`) true false)
  (`TextBlock.SetText` (`/Game/Characters/Components/Interaction/WBP_InteractionHint.HintText` (`self.HintWidget`)) (`self.UnlockFailText`)))

(fn `ShowUnlockHint`
  (`SceneComponent.SetVisibility` (`self.Widget`) true true)
  (`TextBlock.SetText` (`/Game/Characters/Components/Interaction/WBP_InteractionHint.HintText` (`self.HintWidget`)) (`self.LockedText`)))

(fn `UnlockDoor`
  (bind _accesspanelmesh (`self.AccessPanelMesh`))
  (if (not (`self.Unlocked`))
    (set `self.Unlocked` true)
    (`PrimitiveComponent.SetMaterial` _accesspanelmesh 0 (`self.UnlockedStandMat`))
    (`PrimitiveComponent.SetMaterial` _accesspanelmesh 1 (`self.UnlockedMonitorMat`))
    (`GameplayStatics.PlaySound2D` "/Game/Minigames/BugGame/success_low.success_low" 1.0 1.0 0.0 null null false)
    (`self.OnDoorUnlocked`)))

(fn `UnlockWithKey`
  (params (InteractorInventory :type "/Game/Characters/Components/Inventory/InventoryComponent Object Reference (by ref)"))
  (returns (UnlockSuccess :type Boolean))
  (bind _keyitem (`self.KeyItem`))
  (if (`/Game/Characters/Components/Inventory/InventoryComponent.ContainsQuestItem` InteractorInventory (`self.KeyItem`))
    (if (`/Game/Characters/Components/Inventory/QuestItems/QuestItemDataAsset.IsSingleUse` _keyitem)
      (`/Game/Characters/Components/Inventory/InventoryComponent.RemoveQuestItem` (`local.InteractorInventory`) _keyitem))
    (`self.UnlockDoor`)
    (return true)
    (else
      (return false))))

(fn `UserConstructionScript`
  (`PrimitiveComponent.SetMaterial` (`self.SM_Door_01_A`) 0 (`self.Material`))
  (`PrimitiveComponent.SetMaterial` (`self.SM_Door_01_B_Left`) 0 (`self.Material`))
  (`PrimitiveComponent.SetMaterial` (`self.SM_Door_01_C_Right`) 0 (`self.Material`))
  (`PrimitiveComponent.SetMaterial` (`self.SM_Door_01_D`) 0 (`self.Material`)))